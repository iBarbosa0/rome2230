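; AC_Stats is a stats component that tracks Shields and Health and handles damage, healing and death.
; Damage_Stat drains Shields first, then carries any overflow into Health, clamping both and printing the results.
; When Health reaches zero, a DoOnce triggers Death, which calls the OnDeath dispatcher so listeners can react.
; Heal_Stat refills Shields only, leaving Health unchanged.
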(event Custom|Damage_Stat
  (params (Amount :type Float%20%28double-precision%29))
  (Utilities|FlowControl|Sequence
    (:then_0
      ;[1 1 1] Overflow of Damage: For Example- Shields is 30, Damage is 50. So the Result would be -20
      (Variables|Default|SetLeftOverDamage (- (Variables|Default|GetShields) Amount)))
    (:then_1
      (bind _output_get (Variables|Default|SetShields (Math|Float|Clamp(Float) (Variables|Default|GetLeftOverDamage) 0.0 1e+02)))
      (Development|PrintString (Utilities|String|Append "Shields: " (Utilities|String|ToString(Float) _output_get))))
    (:then_2
      (if (< (Math|Float|Sign(Float) (Variables|Default|GetLeftOverDamage)) 0.0)
        (bind _output_get_2 (Variables|Default|SetHealth (Math|Float|Clamp(Float) (- (Variables|Default|GetHealth) (Math|Float|Absolute(Float) (Variables|Default|GetLeftOverDamage))) 0.0 1e+02)))
        (Development|PrintString (Utilities|String|Append "Health: " (Utilities|String|ToString(Float) _output_get_2)))
        ;[1 1 1] If Health is 0 or lower then call the Death Event Dispatcher- Things that are listening can then do actions based on this.
        (if (<= (Variables|Default|GetHealth) 0.0)
          ;;[1 1 1] Can Only Die Once
          (Utilities|FlowControl|DoOnce false
            (:Completed
              (CallFunction|Death))))))))

(event Custom|Death
  ;[1 1 1] If Health is 0 or lower then call the Death Event Dispatcher- Things that are listening can then do actions based on this.
  (Default|CallOnDeath))

(event Custom|Heal_Stat
  (Development|PrintString "AC Stats: Heal")
  (Variables|Default|SetShields 1e+02))