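; Weapon pickup spawner Blueprint that chooses a random weapon pickup type to spawn.
; Its RandomPickUp event picks a random row from WeaponDataTable, stores that row's PickUpClass in PickUpTypeTemp and prints the class name for debugging.
; The construction script only calls the parent's, and this Blueprint contains no spawning logic of its own.
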(event EventRandomPickUp
  (bind _weapondatatable (Variables|Default|GetWeaponDataTable))
  (bind _outrownames (DataTable|GetDataTableRowNames _weapondatatable))
  (bind _returnvalue (Utilities|GetDataTableRow _weapondatatable (.OutItem (Utilities|Array|Random _outrownames)))
    (:then
      (bind _output_get (Variables|Default|SetPickUpType_Temp (.PickUpClass (Utilities|Struct|BreakS_Weapon_Settings _returnvalue))))
      (Development|PrintString (Utilities|String|Append "New Random Weapon To Spawn: " (Utilities|GetClassDisplayName _output_get))))))

(fn ConstructionScript
  (|CallParentFunction))