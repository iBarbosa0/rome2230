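; Base pickup actor that fires once, on authority, when a first-person character overlaps its sphere, then hides and destroys itself after a short delay.
; The overlap event logs the player, calls a server hook and a multi event, then broadcasts the OnPickUp dispatcher.
; The multi event disables collision and calls a local hook.
; Server and local hooks are empty, left for child classes to override with specific pickup behavior.
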(event OnComponentBeginOverlap(Sphere)
  (params (OverlappedComponent :type Primitive%20Component%20Object%20Reference) (OtherActor :type Actor%20Object%20Reference) (OtherComp :type Primitive%20Component%20Object%20Reference) (OtherBodyIndex :type Integer) (bFromSweep :type Boolean) (SweepResult :type Hit%20Result%20Structure%20%28by%20ref%29))
  (bind _asbp_first_person_character (Utilities|Casting|CastToBP_FirstPersonCharacter OtherActor))
  (Networking|SwitchHasAuthority
    (:Authority
      (Utilities|FlowControl|DoOnce false
        (:Completed
          (CallFunction|PickUpOverlap _asbp_first_person_character)
          (Rendering|SetActorHiddenInGame true)
          (Utilities|FlowControl|Delay 0.2)
          (Actor|DestroyActor))))))

(event Custom|PickUp_Overlap
  (params (OverlappingPlayer :type BP%20First%20Person%20Character%20Object%20Reference))
  (Variables|Default|SetOverlappingPlayer OverlappingPlayer)
  (Development|PrintString (Utilities|String|Append "Pick Up Overlap:: Overlapping Player = " (Utilities|GetDisplayName (Variables|Default|GetOverlappingPlayer))))
  (Utilities|FlowControl|Sequence
    (:then_0
      (CallFunction|PickUpOverlapSVR (Variables|Default|GetOverlappingPlayer)))
    (:then_1
      (CallFunction|PickUpOverlapMulti (Variables|Default|GetOverlappingPlayer)))
    (:then_2
      (Default|CallOnPickUp (Variables|Default|GetOverlappingPlayer)))))

(event Custom|PickUp_Overlap_Multi
  (params (OverlappingPlayer :type BP%20First%20Person%20Character%20Object%20Reference))
  (bind _output_get (Variables|Default|SetOverlappingPlayer OverlappingPlayer))
  (Collision|SetActorEnableCollision false)
  (CallFunction|PickUpOverlapLocal _output_get))

(event Custom|PickUp_Overlap_SVR
  (params (OverlappingPlayer :type BP%20First%20Person%20Character%20Object%20Reference))
  ;[1 1 1] These Can Be Overwritten in the Child Classes
)

(event Custom|PickUp_Overlap_Local
  (params (OverlappingPlayer :type BP%20First%20Person%20Character%20Object%20Reference))
  ;[1 1 1] These Can Be Overwritten in the Child Classes
)

(fn ConstructionScript)