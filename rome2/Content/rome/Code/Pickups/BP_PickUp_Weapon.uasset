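; Weapon pickup, built on a parent pickup class, that gives the overlapping player a weapon through their left weapon component using PickUpName.
; On BeginPlay the server looks up PickUpName in the weapon data table, stores the row as WeaponSettings and refreshes the pickup.
; WeaponSettings replicates with an OnRep, so server and clients share one event that sets the name text and skeletal mesh.
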(event Custom|RepEvent_WeaponSettings
  (bind _weaponsettings (Variables|Default|GetWeaponSettings))
  (bind (_weaponname _stats _fx) (Utilities|Struct|BreakS_Weapon_Settings _weaponsettings))
  (Utilities|FlowControl|Sequence
    (:then_0
      (Rendering|Components|TextRender|SetText (Variables|Default|GetTextRender) (Utilities|Text|ToText(Name) _weaponname)))
    (:then_1
      (Components|SkeletalMesh|SetSkeletalMeshAsset (Variables|Default|GetSkeletalMesh) (.Mesh (Utilities|Struct|BreakS_Weapon_Settings_FX _fx))))))

(event EventPickUpOverlapSVR
  (params (OverlappingPlayer :type BP%20First%20Person%20Character%20Object%20Reference))
  (|CallParentFunction OverlappingPlayer)
  (Default|NewWeapon (Variables|/Game/rome/Code/BP_FirstPersonCharacter.BP_FirstPersonCharacter_C|GetWeapon_Left_Comp OverlappingPlayer) (Variables|Default|GetPickUpName)))

(event EventBeginPlay
  (Networking|SwitchHasAuthority
    (:Authority
      (bind _returnvalue (Utilities|GetDataTableRow (Variables|Default|GetWeaponDataTable) (Variables|Default|GetPickUpName))
        (:then
          (Variables|Default|SetWeaponSettings _returnvalue)
          (CallFunction|RefreshPickUp))
        (:RowNotFound
          (Development|PrintString (Utilities|String|Append "Row Not Found: " (Utilities|String|ToString(Name) (Variables|Default|GetPickUpName)))))))))

(event EventRefreshPickUp
  (|CallParentFunction)
  (CallFunction|RepEventWeaponSettings))

(fn ConstructionScript
  (|CallParentFunction))

(fn OnRepWeaponSettings
  (CallFunction|RepEventWeaponSettings))